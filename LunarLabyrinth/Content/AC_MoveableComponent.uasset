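; Moveable component that provides move and rotate actions for a BP_ReflectableObject handed to it through SetDerivedObject.
; Move delegates to the object's own MoveActor, while Rotate adds AngleRot to the relative yaw of its Anchor, keeping roll and pitch.
; Both actions cast the stored object and do nothing for other types.
; GetMovementData, GetRotationData and AddRotation are unimplemented stubs.
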(fn SetDerivedObject
  (params (MoveableObject :type Actor%20Object%20Reference))
  (Variables|Default|SetmoveableObject MoveableObject))

(fn Move
  (bind _asbp_reflectable_object (Utilities|Casting|CastToBP_ReflectableObject (Variables|Default|GetmoveableObject)))
  (Default|MoveActor _asbp_reflectable_object))

(fn Rotate
  (bind _asbp_reflectable_object (Utilities|Casting|CastToBP_ReflectableObject (Variables|Default|GetmoveableObject)))
  (bind _newrot (CallFunction|CalculateNewRotation _asbp_reflectable_object))
  (Transformation|SetRelativeRotation (Variables|/Game/BP_ReflectableObject.BP_ReflectableObject_C|GetAnchor _asbp_reflectable_object) _newrot false false))

(fn CalculateNewRotation
  (params (Actor :type Actor%20Object%20Reference))
  (bind _asbp_reflectable_object (Utilities|Casting|CastToBP_ReflectableObject Actor))
  (return (Math|Rotator|MakeRotator (.Roll (Math|Rotator|BreakRotator (Variables|/Script/Engine.SceneComponent|GetRelativeRotation (Variables|/Game/BP_ReflectableObject.BP_ReflectableObject_C|GetAnchor _asbp_reflectable_object)))) (.Pitch (Math|Rotator|BreakRotator (Variables|/Script/Engine.SceneComponent|GetRelativeRotation (Variables|/Game/BP_ReflectableObject.BP_ReflectableObject_C|GetAnchor _asbp_reflectable_object)))) (+ (.Yaw (Math|Rotator|BreakRotator (Variables|/Script/Engine.SceneComponent|GetRelativeRotation (Variables|/Game/BP_ReflectableObject.BP_ReflectableObject_C|GetAnchor _asbp_reflectable_object)))) (Variables|Default|GetangleRot)))))

(fn GetMovementData)

(fn GetRotationData)