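; Placeable puzzle piece that projects and relays light rays through a reflectable component (ACReflectable), optionally acting as the starting light source.
; Construction binds the component to LightRayAnchor, shows enabled right, rear and left inputs, and sets move/rotate flags and indicators.
; BeginPlay enables query collision on those inputs and starts projection for sources.
; StopHoldObject updates the ray origin if the anchor changed, but samples the old transform immediately before comparing.
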(event EventBeginPlay
  (Utilities|FlowControl|Sequence
    (:then_0
      (if (Variables|Default|GetRightInput)
        (Collision|SetCollisionEnabled (Variables|Default|GetSMC_RightInput) "QueryOnly")))
    (:then_1
      (if (Variables|Default|GetRearInput)
        (Collision|SetCollisionEnabled (Variables|Default|GetSMC_RearInput) "QueryOnly")))
    (:then_2
      (if (Variables|Default|GetLeftInput)
        (Collision|SetCollisionEnabled (Variables|Default|GetSMC_LeftInput) "QueryOnly")))
    (:then_3
      (if (Variables|Default|GetlightSrcStart)
        (Default|StartProjectingLightSource (Variables|Default|GetAC_Reflectable))))))

(event EventTick
  (params (DeltaSeconds :type Float%20%28single-precision%29))
  (CallFunction|IsInteractable))

(event EventStopHoldObject
  (bind _lightrayanchor (Variables|Default|GetLightRayAnchor))
  (Variables|Default|SetoldLoc (Transformation|GetWorldLocation _lightrayanchor))
  (Variables|Default|SetoldFwdVec (Math|Vector|GetForwardVector _lightrayanchor))
  (if (or (Utilities|Operators|NotEqual(!=) (Variables|Default|GetoldLoc) (Transformation|GetWorldLocation _lightrayanchor) 0.0) (Utilities|Operators|NotEqual(!=) (Variables|Default|GetoldFwdVec) (Math|Vector|GetForwardVector _lightrayanchor) 0.0))
    (Default|SetLightSrcLoc (Variables|Default|GetAC_Reflectable))))

(fn ConstructionScript
  (Utilities|FlowControl|Sequence
    (:then_0
      (CallFunction|InitializeReflectableComponent))
    (:then_1
      (Utilities|FlowControl|Sequence
        (:then_0
          (if (Variables|Default|GetRightInput)
            (Rendering|SetVisibility (Variables|Default|GetLightRayNegYInput) true true)))
        (:then_1
          (if (Variables|Default|GetRearInput)
            (Rendering|SetVisibility (Variables|Default|GetLightRayNegXInput) true true)))
        (:then_2
          (if (Variables|Default|GetLeftInput)
            (Rendering|SetVisibility (Variables|Default|GetLightRayYInput) true true)))))
    (:then_2
      (bind _output_get (Variables|Default|SetbMoveable (Variables|Default|GetbCanMove)))
      (Variables|Default|SetbGrabbable _output_get))
    (:then_3
      (Variables|Default|SetbRotateable (Variables|Default|GetbCanRotate)))
    (:then_4
      (if (and (not (Variables|Default|GetbCanMove)) (not (Variables|Default|GetbCanRotate)))
        (Components|StaticMesh|SetStaticMesh (Variables|Default|GetTypeIndicatorStatic) "/Game/LunarLabyrinth/Art/SM_Floor01.SM_Floor01")
        (elif (and (Variables|Default|GetbCanRotate) (not (Variables|Default|GetbCanMove)))
          (Rendering|SetVisibility (Variables|Default|GetTypeIndicatorRotate) true false))))))

(fn InitializeReflectableComponent
  (bind _ac_reflectable (Variables|Default|GetAC_Reflectable))
  (Utilities|FlowControl|Sequence
    (:then_0
      (CallFunction|InitializeMasterReflectableRef))
    (:then_1
      (Default|SetLightSrcMesh _ac_reflectable (Variables|Default|GetLightRayAnchor)))
    (:then_2
      (Default|SetLightSrcLoc _ac_reflectable))
    (:then_3
      (Default|SetOwningActor (Variables|Default|GetAC_Reflectable) self))))

(fn SetReflectableCompLoc
  (bind _ac_reflectable (Variables|Default|GetAC_Reflectable))
  ;[0.01005 0.01042 0 0.906] Set Ray StartPoint
  (Variables|/Game/LunarLabyrinth/Core/Interactables/AC_ReflectableComponent.AC_ReflectableComponent_C|SetrayStartWorldLoc _ac_reflectable (Transformation|GetWorldLocation (Variables|Default|GetLightRayAnchor)))
  (Variables|/Game/LunarLabyrinth/Core/Interactables/AC_ReflectableComponent.AC_ReflectableComponent_C|SetrayStartFwdRot _ac_reflectable (Math|Vector|GetForwardVector (Variables|Default|GetLightRayAnchor))))

(fn IsInteractable
  (return true))