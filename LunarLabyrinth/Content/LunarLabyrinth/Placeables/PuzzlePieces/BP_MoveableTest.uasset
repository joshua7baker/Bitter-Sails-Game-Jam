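; BP_MoveableTest is a test puzzle piece for Lunar Labyrinth that moves in 100-unit steps and rotates.
; StartMoveObject forwards a direction to ACMoveableComp, while MoveObjectPosition sets an axis-aligned target from the current location.
; A timeline lerps the actor's current location toward that target without sweeping.
; A separate timeline drives the Anchor's relative yaw by its track value times 90 degrees.
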(event EventBeginPlay
  (|CallParentFunction))

(event Collision|EventActorBeginOverlap
  (params (OtherActor :type Actor%20Object%20Reference))
  (|CallParentFunction OtherActor) ; This node is disabled and will not be called.\nDrag off pins to build functionality.
)

(event EventTick
  (params (DeltaSeconds :type Float%20%28single-precision%29))
  (|CallParentFunction DeltaSeconds) ; This node is disabled and will not be called.\nDrag off pins to build functionality.
)

(event EventStartMoveObject
  (params (moveDirectionIn :type Vector :default "0, 0, 0"))
  (Default|MoveObject (Variables|Default|GetAC_MoveableComp) moveDirectionIn))

(event EventMoveObjectPosition
  (params (EDirection :type MovementDirection%20Enum :default "NewEnumerator0"))
  (bind _returnvalue (Transformation|GetActorLocation))
  (switch Utilities|FlowControl|Switch|SwitchonMovementDirection EDirection
    (:NewEnumerator0
      (Variables|Default|SettargetLoc (+ _returnvalue "100.000000,0.000000,0.000000"))
      (bind _movementtrack (Timeline|MovementTimeline Play)
        (:Update
          (Transformation|SetActorLocation (Math|Vector|Lerp(Vector) (Transformation|GetActorLocation) (Variables|Default|GettargetLoc) _movementtrack) false false))))
    (:NewEnumerator1
      (Variables|Default|SettargetLoc (- _returnvalue "100.000000,0.000000,0.000000"))
      (Timeline|MovementTimeline Play))
    (:NewEnumerator2
      (Variables|Default|SettargetLoc (- _returnvalue "0.000000,100.000000,0.000000"))
      (Timeline|MovementTimeline Play))
    (:NewEnumerator3
      (Variables|Default|SettargetLoc (+ _returnvalue "0.000000,100.000000,0.000000"))
      (Timeline|MovementTimeline Play))))

(event EventStartRotateObject
  (bind _movementtrack (Timeline|rotationTimeline Play)
    (:Update
      (Transformation|SetRelativeRotation (Variables|Default|GetAnchor) (Math|Rotator|MakeRotator 0.0 0.0 (* _movementtrack 9e+01)) false false))))

(fn ConstructionScript
  (|CallParentFunction))