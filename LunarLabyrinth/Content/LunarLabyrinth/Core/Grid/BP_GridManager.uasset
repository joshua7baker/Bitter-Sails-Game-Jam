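; BP_GridManager is an actor that builds a square grid of BP_Gridcell actors and provides nearest-cell position lookup.
; On BeginPlay, PopulateGrid spawns cells in nested X/Y loops at a fixed spacing and stores them in GridArray.
; The world offset is zeroed and its centering calculation is unused, so the grid extends from the world origin.
; Getclosestgrid linearly scans the array and returns the cell location closest to a given position.
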(event EventBeginPlay
  (CallFunction|PopulateGrid))

(event Collision|EventActorBeginOverlap
  (params (OtherActor :type Actor%20Object%20Reference)))

(event EventTick
  (params (DeltaSeconds :type Float%20%28single-precision%29)))

(fn ConstructionScript)

(fn PopulateGrid
  (bind _worldgridside (Variables|Default|GetWorldgridside))
  (Utilities|Array|Clear (Variables|Default|GetGridArray))
  (LocalVariables|Setworldoffset 0.0)
  ;[1 1 1] Y loop
  (for _index (range 0 (- (Variables|Default|GetGridsize) 1))
    ;[1 1 1] X loop
    (for _index_2 (range 0 (- (Variables|Default|GetGridsize) 1))
      (bind _returnvalue (Game|SpawnActorfromClass "/Game/LunarLabyrinth/Core/Grid/BP_Gridcell.BP_Gridcell_C" (Math|Transform|MakeTransform (Math|Vector|MakeVector (Math|Conversions|ToFloat(Integer) (- (* _index_2 _worldgridside) (Math|Float|Truncate (LocalVariables|Getworldoffset)))) (Math|Conversions|ToFloat(Integer) (- (* _worldgridside _index) (Math|Float|Truncate (LocalVariables|Getworldoffset)))) 0.0)) "AlwaysSpawn" "MultiplyWithRoot" 0 0))
      (Utilities|Array|Add (Variables|Default|GetGridArray) _returnvalue))))

(fn Getclosestgrid
  (params (Inposition :type Vector))
  (bind _gridarray (Variables|Default|GetGridArray))
  (bind _output (Utilities|Array|Get(acopy) _gridarray))
  (bind _returnvalue (Transformation|GetActorLocation _output))
  ;[1 1 1] i knoww i need to learn how to organize bps
  (LocalVariables|Setclosest%20position _returnvalue)
  (LocalVariables|Setclosest%20distance (Math|Vector|Distance(Vector) Inposition _returnvalue))
  (for _array_element (Variables|Default|GetGridArray)
    (if (< (Math|Vector|Distance(Vector) (Transformation|GetActorLocation _array_element) Inposition) (LocalVariables|Getclosest%20distance))
      (LocalVariables|Setclosest%20position (Transformation|GetActorLocation _array_element))
      (LocalVariables|Setclosest%20distance (Math|Vector|Distance(Vector) (Transformation|GetActorLocation _array_element) Inposition))))
  (return (LocalVariables|Getclosest%20position)))