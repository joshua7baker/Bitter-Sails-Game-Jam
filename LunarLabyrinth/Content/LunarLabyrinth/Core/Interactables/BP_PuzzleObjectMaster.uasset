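; BP_PuzzleObjectMaster is the base Blueprint for puzzle objects that the player can grab or rotate.
; Its construction script sets the mesh, derives interaction flags, always adds a reflectable component, and adds the moveable component only when Rotateable.
; Primary interaction grabs through that component, notifies the controller and levitates the object via timeline into a flip-flopped floating bob; secondary interaction starts rotation.
; Subclasses implement BPI_Interactable themselves.
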(event Custom|LevitateMovableObject
  (Default|SetCanInteract (Variables|Default|Getplayer_BP) false)
  ;[0 0 0] Levitate Object to start floating
  (bind _output_get (Variables|Default|SetstartMoveableLoc (Transformation|GetActorLocation)))
  (Variables|Default|SetbInteractable false)
  (Audio|PlaySoundatLocation "/Game/LunarLabyrinth/Audio/block_movment_lift_noise__1_.block_movment_lift_noise__1_" _output_get "0, 0, 0" 1.0 1.0 0.0 0 0 0 0)
  (bind _raiseobjecttrack (Timeline|LevitateObject PlayFromStart)
    (:Update
      (Transformation|SetActorLocation (Math|Vector|Lerp(Vector) (Variables|Default|GetstartMoveableLoc) (Math|Vector|MakeVector (.X (Math|Vector|BreakVector (Variables|Default|GetstartMoveableLoc))) (.Y (Math|Vector|BreakVector (Variables|Default|GetstartMoveableLoc))) (+ (.Z (Math|Vector|BreakVector (Variables|Default|GetstartMoveableLoc))) 1e+02)) _raiseobjecttrack) false false))
    (:Finished
      (Variables|Default|SetbFloating true)
      (Variables|Default|SetbInteractable true)
      (CallFunction|StartFloating))))

(event Custom|StartFloating
  (bind _returnvalue (Transformation|GetActorLocation))
  (bind (_x _y _z) (Math|Vector|BreakVector _returnvalue))
  ;[0 0 0] Floating Animation
  (Variables|Default|SetendFloatLoc (Math|Vector|MakeVector _x _y (+ _z 1e+01)))
  (bind _floatobjecttrack (Timeline|FloatObjectAround PlayFromStart)
    (:Update
      (Transformation|SetActorLocation (Math|Vector|Lerp(Vector) (Transformation|GetActorLocation) (Variables|Default|GetendFloatLoc) _floatobjecttrack) false false))
    (:Finished
      (if (Variables|Default|GetbFloating)
        (bind _output_get (Variables|Default|SetstartMoveableLoc (Transformation|GetActorLocation)))
        (Utilities|FlowControl|FlipFlop
          (:A
            (Variables|Default|SetendFloatLoc (Math|Vector|MakeVector (.X (Math|Vector|BreakVector _output_get)) (.Y (Math|Vector|BreakVector _output_get)) (- (.Z (Math|Vector|BreakVector _output_get)) 1e+01))))
          (:B
            (Variables|Default|SetendFloatLoc (Math|Vector|MakeVector (.X (Math|Vector|BreakVector _output_get)) (.Y (Math|Vector|BreakVector _output_get)) (+ (.Z (Math|Vector|BreakVector _output_get)) 1e+01)))))
        (CallFunction|ResumeFloating)))))

(event Custom|StopLevitating
  (bind _startmoveableloc (Variables|Default|GetstartMoveableLoc))
  (bind (_x _y _z) (Math|Vector|BreakVector _startmoveableloc))
  ;[0 0 0] Levitate Object to start floating
  (bind _raiseobjecttrack (Timeline|LevitateObject Stop)
    (:Update
      (Transformation|SetActorLocation (Math|Vector|Lerp(Vector) _startmoveableloc (Math|Vector|MakeVector _x _y (+ _z 1e+02)) _raiseobjecttrack) false false))
    (:Finished
      (Variables|Default|SetbFloating true)
      (Variables|Default|SetbInteractable true)
      (CallFunction|StartFloating))))

(event Custom|ResumeFloating
  ;[0 0 0] Floating Animation
  (bind _floatobjecttrack (Timeline|FloatObjectAround ReverseFromEnd)
    (:Update
      (Transformation|SetActorLocation (Math|Vector|Lerp(Vector) (Transformation|GetActorLocation) (Variables|Default|GetendFloatLoc) _floatobjecttrack) false false))
    (:Finished
      (if (Variables|Default|GetbFloating)
        (bind _output_get (Variables|Default|SetstartMoveableLoc (Transformation|GetActorLocation)))
        (Utilities|FlowControl|FlipFlop
          (:A
            (Variables|Default|SetendFloatLoc (Math|Vector|MakeVector (.X (Math|Vector|BreakVector _output_get)) (.Y (Math|Vector|BreakVector _output_get)) (- (.Z (Math|Vector|BreakVector _output_get)) 1e+01))))
          (:B
            (Variables|Default|SetendFloatLoc (Math|Vector|MakeVector (.X (Math|Vector|BreakVector _output_get)) (.Y (Math|Vector|BreakVector _output_get)) (+ (.Z (Math|Vector|BreakVector _output_get)) 1e+01)))))
        (CallFunction|ResumeFloating)))))

(event Custom|StopFloating
  ;[0 0 0] Floating Animation
  ;;[1 1 1] Call this once object has been moved
  (Variables|Default|SetbFloating false)
  (bind _floatobjecttrack (Timeline|FloatObjectAround Stop)
    (:Update
      (Transformation|SetActorLocation (Math|Vector|Lerp(Vector) (Transformation|GetActorLocation) (Variables|Default|GetendFloatLoc) _floatobjecttrack) false false))
    (:Finished
      (if (Variables|Default|GetbFloating)
        (bind _output_get (Variables|Default|SetstartMoveableLoc (Transformation|GetActorLocation)))
        (Utilities|FlowControl|FlipFlop
          (:A
            (Variables|Default|SetendFloatLoc (Math|Vector|MakeVector (.X (Math|Vector|BreakVector _output_get)) (.Y (Math|Vector|BreakVector _output_get)) (- (.Z (Math|Vector|BreakVector _output_get)) 1e+01))))
          (:B
            (Variables|Default|SetendFloatLoc (Math|Vector|MakeVector (.X (Math|Vector|BreakVector _output_get)) (.Y (Math|Vector|BreakVector _output_get)) (+ (.Z (Math|Vector|BreakVector _output_get)) 1e+01)))))
        (CallFunction|ResumeFloating)))))

(event EventStartInteract
  (params (playerInteracting :type BP%20Third%20Person%20Character%20Object%20Reference) (bPrimaryInteract :type Boolean) (bSecondaryInteract :type Boolean) (bKeyHeld :type Boolean))
  (Variables|Default|Setplayer_BP playerInteracting)
  (if (or (Variables|Default|GetbMoveable) (Variables|Default|GetbRotateable))
    ;[0.5938 0 0.1405] Change this to a switch on input enum
    (if bPrimaryInteract
      (if (Variables|Default|GetbGrabbable)
        (Default|SetHoldingObject (Variables|Default|Getplayer_BP) true self)
        (Class|BPIMoveable|GrabObject(Message) (Variables|Default|GetAC_MoveableComp))
        (if (Utilities|DoesObjectImplementInterface (Pawn|GetController (Variables|Default|Getplayer_BP)) "/Game/LunarLabyrinth/Core/Interactables/BPI_Interactable.BPI_Interactable_C")
          (Class|BPIInteractable|StartHoldObject(Message) (Pawn|GetController (Variables|Default|Getplayer_BP)))
          (CallFunction|LevitateMovableObject)))
      (elif bSecondaryInteract
        (Class|BPIMoveable|StartRotateObject(Message) self)))))

(fn ConstructionScript
  (Utilities|FlowControl|Sequence
    (:then_0
      (CallFunction|InitializePuzzleObj))
    (:then_1
      (CallFunction|CheckInteractable))
    (:then_2
      (CallFunction|CheckMoveable))
    (:then_3
      (CallFunction|InitializeMasterReflectableRef))))

(fn CheckInteractable
  ;[0.2805 0.2917 0.2188] Interface is manually implemented in the sub classes of PuzzleObjectMaster
  (Variables|Default|SetbInteractable (Utilities|DoesObjectImplementInterface self "/Game/LunarLabyrinth/Core/Interactables/BPI_Interactable.BPI_Interactable_C")))

(fn InitializePuzzleObj
  ;[0.01005 0.01042 0 0.906] Set ReflectableComponent Mesh
  (Components|StaticMesh|SetStaticMesh (Variables|Default|GetModel) (Variables|Default|GetobjModel)))

(fn CheckMoveable
  (if (Variables|Default|GetbMoveable)
    (Variables|Default|SetbGrabbable true))
  (if (Variables|Default|GetbRotateable)
    ;[0.01005 0.01042 0 0.906] Add & Init Moveable Comp
    (bind _returnvalue (AddComponent|AddACMoveableComponent))
    (bind _output_get (Variables|Default|SetAC_MoveableComp _returnvalue))
    (Default|SetDerivedObject _output_get self)))

(fn IsMovable
  (params (NewParam :type Boolean))
  (return (Variables|Default|GetbMoveable)))

(fn IsRotatable
  (return (Variables|Default|GetbRotateable)))

(fn InitializeMasterReflectableRef
  (bind _returnvalue (AddComponent|AddACReflectableComponent))
  (Variables|Default|SetAC_Reflectable _returnvalue))

(fn IsInteractable
  (return (Variables|Default|GetbInteractable)))