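; BP_splinecomponent is a construction-time spline placement tool that repeats a chosen static mesh along a spline path.
; The construction script derives spacing from the mesh's bounding-box X size plus an offset, then divides the spline length by it to get the instance count.
; It adds instances to an InstancedStaticMesh at local spline positions, with zero rotation and unit scale, so meshes do not follow the curve's direction.
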(event EventBeginPlay)

(event Collision|EventActorBeginOverlap
  (params (OtherActor :type Actor%20Object%20Reference)))

(event EventTick
  (params (DeltaSeconds :type Float%20%28single-precision%29)))

(fn ConstructionScript
  (bind _placedmesh (Variables|Default|GetPLACEDMESH))
  (bind _returnvalue (StaticMesh|GetBoundingBox _placedmesh))
  (bind (_min _max) (Utilities|Struct|BreakBox _returnvalue))
  ;[1 1 1] BASIC SPLINE
  (Components|StaticMesh|SetStaticMesh (Variables|Default|GetInstancedStaticMesh) (Variables|Default|GetPLACEDMESH))
  (bind _output_get (Variables|Default|SetSPACING (+ (.X (Math|Vector|BreakVector (- _max _min))) (Variables|Default|GetOFFSET))))
  (bind _output_get_2 (Variables|Default|SetNUMBER%20OF%20INSTANCES (Math|Float|Floor (/ (Spline|GetSplineLength (Variables|Default|GetSpline)) _output_get))))
  (for _index (range 0 _output_get_2)
    (Components|InstancedStaticMesh|AddInstance (Variables|Default|GetInstancedStaticMesh) (Math|Transform|MakeTransform (Spline|GetLocationatDistanceAlongSpline (Variables|Default|GetSpline) (* _index (Variables|Default|GetSPACING)) "Local")) false)))