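; BP_Clickable is an interactable component that gives its owning actor mouse hover and click feedback.
; On begin play it binds the owner's click event and, if a static mesh component exists, caches it and binds cursor-over events.
; Hovering toggles the mesh's custom depth rendering, while each click flips its first material between ArrowMaterial and BasicAsset01.
; The inPlacementMode event destroys the component.
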(event Custom|OnMouseClick
  (params (TouchedActor :type Actor%20Object%20Reference) (ButtonPressed :type Key%20Structure :default "None"))
  (bind _static_mesh_reference (Variables|Default|Getstatic%20mesh%20reference))
  (bind _output_get (Variables|Default|Setis%20clicked%20? (not (Variables|Default|Getis%20clicked%20?))))
  (Utilities|IsValid (Variables|Default|Getstatic%20mesh%20reference)
    (:Is%20Valid
      (if _output_get
        (Rendering|Material|SetMaterial _static_mesh_reference 0 "/Engine/VREditor/UI/ArrowMaterial.ArrowMaterial")
        (else
          (Rendering|Material|SetMaterial _static_mesh_reference 0 "/Engine/MapTemplates/Materials/BasicAsset01.BasicAsset01"))))))

(event Custom|inPlacementMode
  (Components|DestroyComponent))

(event Custom|OnMouseHover
  (params (TouchedActor :type Actor%20Object%20Reference))
  (Rendering|SetRenderCustomDepth (Variables|Default|Getstatic%20mesh%20reference) true))

(event Custom|OnMouseHoverOver
  (params (TouchedActor :type Actor%20Object%20Reference))
  (Rendering|SetRenderCustomDepth (Variables|Default|Getstatic%20mesh%20reference) false))

(event EventBeginPlay
  (bind _returnvalue (Components|GetOwner))
  (bind _returnvalue_2 (Actor|GetComponentbyClass _returnvalue "/Script/Engine.StaticMeshComponent"))
  (EventDispatchers|BindEventtoOnClicked _returnvalue (delegate Custom|OnMouseClick))
  (Utilities|IsValid _returnvalue_2
    (:Is%20Valid
      (Variables|Default|Setstatic%20mesh%20reference _returnvalue_2)
      (EventDispatchers|BindEventtoOnBeginCursorOver _returnvalue (delegate Custom|OnMouseHover))
      (EventDispatchers|BindEventtoOnEndCursorOver _returnvalue (delegate Custom|OnMouseHoverOver)))))