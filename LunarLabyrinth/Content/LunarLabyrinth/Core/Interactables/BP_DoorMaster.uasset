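; BP_DoorMaster is a door in Lunar Labyrinth that opens as a sinking puzzle door and, when flagged FinalDoor, closes by swinging.
; Open plays a sound and lerps the actor from its current location toward a lowered point set in the construction script, then disables model collision.
; Close rotates the Anchor via timeline-driven RInterpTo to a yaw target from SetDoorTargetRot; the matching swing-open branch is unconnected.
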(event Custom|Open
  (Audio|PlaySoundatLocation "/Game/LunarLabyrinth/Audio/door_sound.door_sound" (Variables|Default|GetstartDoorLoc) "0, 0, 0" 0.3 1.0 0.0 0 0 0 0)
  ;[0 0 0] Open puzzle door
  (Components|Timeline|SetPlayRate (Variables|Default|GetTimeline) 1.0)
  (bind _anchorrotate (Timeline|Timeline PlayFromStart)
    (:Update
      (Transformation|SetActorLocation (Math|Vector|Lerp(Vector) (Transformation|GetActorLocation) (Variables|Default|GetendDoorLoc) _anchorrotate) false false))
    (:Finished
      (Collision|SetCollisionEnabled (Variables|Default|GetModel) "NoCollision"))))

(event Custom|Close
  (if (Variables|Default|GetbFinalDoor)
    ;[0 0 0] Open Close regular Door
    (CallFunction|SetDoorTargetRot false)
    (bind _anchorrotate (Timeline|Open/Close%20Door PlayFromStart)
      (:Update
        (Transformation|SetRelativeRotation (Variables|Default|GetAnchor) (Math|Interpolation|RInterpTo (Variables|/Script/Engine.SceneComponent|GetRelativeRotation (Variables|Default|GetAnchor)) (Variables|Default|GetendDoorRot) _anchorrotate 1.0) false false)))))

(fn ConstructionScript
  (bind _returnvalue (Transformation|GetActorLocation))
  (bind (_x _y _z) (Math|Vector|BreakVector _returnvalue))
  (Variables|Default|SetendDoorLoc (Math|Vector|MakeVector _x _y (- _z 3e+02))))

(fn SetDoorTargetRot
  (params (bOpening :type Boolean))
  (bind _startdoorrot (Variables|Default|GetstartDoorRot))
  (bind _startdoorrot_2 (Variables|Default|GetstartDoorRot))
  (bind (_roll _pitch _yaw) (Math|Rotator|BreakRotator _startdoorrot))
  (bind (_roll_2 _pitch_2 _yaw_2) (Math|Rotator|BreakRotator _startdoorrot_2))
  (if bOpening
    (Variables|Default|SetendDoorRot (Math|Rotator|MakeRotator _roll_2 _pitch_2 (+ _yaw_2 9e+01)))
    (else
      (Variables|Default|SetendDoorRot (Math|Rotator|MakeRotator _roll _pitch (- _yaw 9e+01))))))