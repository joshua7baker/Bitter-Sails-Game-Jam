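; Actor component for a light-ray reflection puzzle that chains reflectable objects from a light source and opens doors.
; A fast looping timer line-traces from the output mesh's cached transform, drawing only a debug line.
; Hitting a light-input component connects a stationary reflectable, which starts its own trace, or opens a door.
; Losing that hit or looping back to the source recursively disconnects the downstream chain; sound nodes are unwired.
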(event Custom|LineTraceForConnection
  (bind _raystartworldloc (Variables|Default|GetrayStartWorldLoc))
  ;[0.1667 0.06932 0] Reflective Light Ray Functionality
  (bind _outhit (Collision|LineTraceByChannel _raystartworldloc (+ _raystartworldloc (* (Variables|Default|GetrayStartFwdRot) 1.25e+03)) "TraceTypeQuery4" false 0 "ForOneFrame" true "(R=1.000000,G=0.000000,B=0.000000,A=1.000000)" "(R=0.000000,G=0.000000,B=0.000000,A=0.000000)"))
  (if (.bBlockingHit (Collision|BreakHitResult _outhit))
    (Utilities|Casting|CastToSMC_LightRayInput (.HitComponent (Collision|BreakHitResult _outhit))
      (:then
        (bind _asbp_reflectable_object (Utilities|Casting|CastToBP_ReflectableObject (.HitActor (Collision|BreakHitResult _outhit)))
          (:then
            (if (!= (Variables|Default|GetconnectedReflectableObj) _asbp_reflectable_object)
              (bind _output_get (Variables|Default|SethitReflectableObj _asbp_reflectable_object))
              (if (== _output_get (Variables|Default|GetsrcReflectableObj))
                (CallFunction|TriggerDisconnect)
                (elif (not (Variables|/Game/LunarLabyrinth/Core/Interactables/BP_PuzzleObjectMaster.BP_PuzzleObjectMaster_C|GetbMoving (Variables|Default|GethitReflectableObj)))
                  (bind _output_get_2 (Variables|Default|SetconnectedReflectableObj (Variables|Default|GethitReflectableObj)))
                  (CallFunction|Connect (Variables|/Game/LunarLabyrinth/Core/Interactables/BP_PuzzleObjectMaster.BP_PuzzleObjectMaster_C|GetAC_Reflectable _output_get_2) (Variables|Default|GetsrcReflectableObj))))))
          (:CastFailed
            (bind _asbp_door_master (Utilities|Casting|CastToBP_DoorMaster (.HitActor (Collision|BreakHitResult _outhit))))
            (Default|Open _asbp_door_master))))
      (:CastFailed
        (Variables|Default|GetconnectedReflectableObj :!label _label
          (:then
            (CallFunction|TriggerDisconnect)
            (Variables|Default|SetconnectedReflectableObj 0))
          (:else))))
    (else
      (goto _label))))

(event Custom|StartReflectingLightRay
  ;[0.1667 0.06932 0] Reflective Light Ray Functionality
  (if (Variables|Default|GetbConnected)
    (bind _returnvalue (Utilities|Time|SetTimerbyEvent (delegate Custom|LineTraceForConnection) 0.01 true))))

(event Custom|StopReflectingLightRay
  ;[0.1667 0.06932 0] Reflective Light Ray Functionality
  (Utilities|Time|ClearandInvalidateTimerbyHandle (stale Custom|StartReflectingLightRay _returnvalue)))

(event Custom|TriggerDisconnect
  ;[0.1979 0.0633 0.05542 0.906] Disconnect Actor if connected
  (Utilities|IsValid (Variables|Default|GetconnectedReflectableObj)
    (:Is%20Valid
      ;;[1 1 1] Disconnect any chain connected objects
      (CallFunction|DisconnectChain (Variables|/Game/LunarLabyrinth/Core/Interactables/BP_PuzzleObjectMaster.BP_PuzzleObjectMaster_C|GetAC_Reflectable (Variables|Default|GetconnectedReflectableObj)))
      (Variables|Default|SetconnectedReflectableObj 0))))

(event Custom|StartProjectingLightSource
  ;[0.1667 0.06932 0] Reflective Light Ray Functionality
  (bind _returnvalue (Utilities|Time|SetTimerbyEvent (delegate Custom|LineTraceForConnection) 0.01 true)))

(event EventBeginPlay
  ;[1 1 1] Begin Play
  (if (Variables|Default|GetbSourceStart)
    (CallFunction|StartProjectingLightSource)))

(fn Connect
  (params (OwningActor :type BP%20Reflectable%20Object%20Object%20Reference))
  (Variables|Default|SetsrcReflectableObj OwningActor)
  (if (not (Variables|Default|GetbConnected))
    (Variables|Default|SetbConnected true)
    (CallFunction|StartReflectingLightRay)))

(fn DisconnectChain
  (Utilities|FlowControl|Sequence
    (:then_0
      (Variables|Default|SetbConnected false)
      (Utilities|IsValid (Variables|Default|GetconnectedReflectableObj)
        (:Is%20Valid
          (if (!= (Variables|/Game/LunarLabyrinth/Core/Interactables/BP_PuzzleObjectMaster.BP_PuzzleObjectMaster_C|GetAC_Reflectable (Variables|Default|GetconnectedReflectableObj)) (Variables|/Game/LunarLabyrinth/Core/Interactables/BP_PuzzleObjectMaster.BP_PuzzleObjectMaster_C|GetAC_Reflectable (Variables|Default|GetsrcReflectableObj)))
            (CallFunction|DisconnectChain (Variables|/Game/LunarLabyrinth/Core/Interactables/BP_PuzzleObjectMaster.BP_PuzzleObjectMaster_C|GetAC_Reflectable (Variables|Default|GetconnectedReflectableObj)))))))
    (:then_1
      (CallFunction|StopReflectingLightRay)
      (Variables|Default|SetconnectedReflectableObj 0))))

(fn SetLightSrcLoc
  (bind _lightrayoutputsm (Variables|Default|GetlightRayOutputSM))
  ;[0.01005 0.01042 0 0.906] Set Ray StartPoint
  (Variables|Default|SetrayStartWorldLoc (Transformation|GetWorldLocation _lightrayoutputsm))
  (Variables|Default|SetrayStartFwdRot (Math|Vector|GetForwardVector _lightrayoutputsm)))

(fn SetLightSrcMesh
  (params (lightRayOutputSM :type Static%20Mesh%20Component%20Object%20Reference))
  (Variables|Default|SetlightRayOutputSM lightRayOutputSM))

(fn SetLightSrcRot
  (params (NewRot :type Rotator))
  ;[0.01005 0.01042 0 0.906] Set Ray StartPoint
  (Transformation|SetRelativeRotation (Variables|Default|GetlightRayOutputSM) NewRot false false))

(fn SetOwningActor
  (params (Actor :type BP%20Reflectable%20Object%20Object%20Reference))
  (Variables|Default|SetsrcReflectableObj Actor))

(fn IsConnectable
  (bind _output_get (Variables|Default|SetbConnectable (Variables|Default|GetbConnectable)))
  (return _output_get))