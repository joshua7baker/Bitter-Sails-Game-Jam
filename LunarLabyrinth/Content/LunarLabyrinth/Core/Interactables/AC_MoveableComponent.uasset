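; Actor component for moveable puzzle objects that forwards move and rotate requests to its assigned MoveableObject.
; MoveObject converts a direction into a four-way enum, X taking priority, sets IsMoving and messages the object; RotateObject sends its message unless IsRotating.
; Helpers snap directions to one XY axis and step a BP_PuzzleObjectMaster's Anchor yaw by AngleRot.
; GrabObject and the data getters are empty, and IsInteractable returns false.
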(event EventGrabObject
  (params (interatingActor :type BP%20Third%20Person%20Character%20Object%20Reference))
  ;[0.1713 0.2769 0.3854] Grab Obj
)

(event EventMoveObject
  (params (moveDirectionIn :type Vector :default "0, 0, 0"))
  (bind (_x _y) (Math|Vector|BreakVector moveDirectionIn))
  ;[0.1713 0.2769 0.3854] Move Object
  (if (not (Variables|Default|GetbIsMoving))
    (if (!= _x 0.0)
      (if (< _x 0.0)
        (Variables|Default|SetEMovementDirection "NewEnumerator2")
        (else
          (Variables|Default|SetEMovementDirection "NewEnumerator3")))
      (elif (> _y 0.0)
        (Variables|Default|SetEMovementDirection "NewEnumerator0")
        (else
          (Variables|Default|SetEMovementDirection "NewEnumerator1"))))
    (Development|PrintString "Hello")
    (Variables|Default|SetbIsMoving true)
    (Class|BPIMoveable|MoveObjectPosition(Message) (Variables|Default|GetmoveableObject) (Variables|Default|GetEMovementDirection))))

(event EventRotateObject
  ;[0.1713 0.2769 0.3854] Rotate Object
  (if (not (Variables|Default|GetbIsRotating))
    (Class|BPIMoveable|StartRotateObject(Message) (Variables|Default|GetmoveableObject))))

(fn SetDerivedObject
  (params (MoveableObject :type Actor%20Object%20Reference))
  (Variables|Default|SetmoveableObject MoveableObject))

(fn Rotate
  (bind _asbp_puzzle_object_master (Utilities|Casting|CastToBP_PuzzleObjectMaster (Variables|Default|GetmoveableObject)))
  (bind _newrot (CallFunction|CalculateNewRotation _asbp_puzzle_object_master))
  (Transformation|SetRelativeRotation (Variables|/Game/LunarLabyrinth/Core/Interactables/BP_PuzzleObjectMaster.BP_PuzzleObjectMaster_C|GetAnchor _asbp_puzzle_object_master) _newrot false false))

(fn CalculateNewRotation
  (params (Actor :type BP%20Puzzle%20Object%20Master%20Object%20Reference))
  (bind _anchor (Variables|/Game/LunarLabyrinth/Core/Interactables/BP_PuzzleObjectMaster.BP_PuzzleObjectMaster_C|GetAnchor Actor))
  (bind _relativerotation (Variables|/Script/Engine.SceneComponent|GetRelativeRotation _anchor))
  (bind (_roll _pitch _yaw) (Math|Rotator|BreakRotator _relativerotation))
  (return (Math|Rotator|MakeRotator _roll _pitch (+ _yaw (Variables|Default|GetangleRot)))))

(fn GetMovementData)

(fn GetRotationData)

(fn GetClosestSingleXYVector
  (params (directionIn :type Vector))
  (bind (_x _y) (Math|Vector|BreakVector directionIn))
  (Variables|Default|SetstartXInput _x)
  (Variables|Default|SetstartYInput _y)
  (if (> (- (|((round((direction/90)))*90) _x) (Variables|Default|GetstartXInput)) (- (|((round((direction/90)))*90) _y) (Variables|Default|GetstartYInput)))
    (Variables|Default|SetmoveDirection (Math|Vector|MakeVector (Variables|Default|GetstartXInput) 0.0 0.0))
    (else
      (Variables|Default|SetmoveDirection (Math|Vector|MakeVector 0.0 (Variables|Default|GetstartYInput) 0.0))))
  (return (Variables|Default|GetmoveDirection)))

(fn IsInteractable
  (return false))