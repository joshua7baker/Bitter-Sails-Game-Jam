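; Player controller that forwards move and interact input to BP_ThirdPersonCharacter and runs a grid-based placement mode for puzzle objects.
; Starting a hold freezes character movement and spawns a preview actor, which follows a mouse trace each tick, snapped to BP_GridManager's closest cell.
; Left click destroys the preview and messages the character's held interactable to move there.
; Physics-handle grab and validity-checked spawn functions also exist but are not called here.
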(event Input|EnhancedActionEvents|EnhancedInputActionIA_Interact
  (params (ActionValue :type Boolean) (ElapsedSeconds :type Float%20%28double-precision%29) (TriggeredSeconds :type Float%20%28double-precision%29) (InputAction :type Input%20Action%20Object%20Reference :default "/Game/LunarLabyrinth/Core/Characters/Player/Input/Actions/IA_Interact.IA_Interact"))
  ;[0.09896 0.02986 0] Primary Interact Input
  (Default|ReceiveInteractInput (Variables|Default|GetBP_PlayerCharacter)))

(event Input|EnhancedActionEvents|EnhancedInputActionIA_Move
  (params (ActionValue :type Vector%202D%20Structure) (ElapsedSeconds :type Float%20%28double-precision%29) (TriggeredSeconds :type Float%20%28double-precision%29) (InputAction :type Input%20Action%20Object%20Reference :default "/Game/LunarLabyrinth/Core/Characters/Player/Input/Actions/IA_Move.IA_Move"))
  ;[0.09896 0.02986 0] Movement
  (Default|ReceiveMovementInput (Variables|Default|GetBP_PlayerCharacter) (.x ActionValue) (.y ActionValue)))

(event Input|EnhancedActionEvents|EnhancedInputActionIA_SecondaryInteract
  (params (ActionValue :type Boolean) (ElapsedSeconds :type Float%20%28double-precision%29) (TriggeredSeconds :type Float%20%28double-precision%29) (InputAction :type Input%20Action%20Object%20Reference :default "/Game/LunarLabyrinth/Core/Characters/Player/Input/Actions/IA_SecondaryInteract.IA_SecondaryInteract"))
  ;[0.09896 0.02986 0] Secondary Interact Input
  (Default|ReceiveSecondInteractInput (Variables|Default|GetBP_PlayerCharacter)))

(event EventStopHoldObject
  (bind _bp_playercharacter (Variables|Default|GetBP_PlayerCharacter))
  ;[0.09896 0.02986 0] Placement Mode: called from Puzzle Object Master
  (Default|SetHoldingObject _bp_playercharacter false)
  (Default|SetPlacementMode _bp_playercharacter false)
  (Components|Activation|Activate (Variables|/Script/Engine.Character|GetCharacterMovement (Variables|Default|GetBP_PlayerCharacter)) true))

(event EventBeginPlay
  ;[0.05098 0.02337 0.02337] Initialization
  (Utilities|FlowControl|Sequence
    (:then_0
      (bind _asbp_third_person_character (Utilities|Casting|CastToBP_ThirdPersonCharacter (Game|GetPlayerCharacter 0)))
      (Variables|Default|SetBP_PlayerCharacter _asbp_third_person_character))
    (:then_1
      (Default|SetInputMapping (Variables|Default|GetBP_PlayerCharacter)))))

(event EventTick
  (params (DeltaSeconds :type Float%20%28single-precision%29))
  (if (Variables|Default|GetisPlacementModeEnabled)
    (Variables|Default|GetploppableActor
      (:then
        (CallFunction|UpdatePlacement))
      (:else))))

(event EventStartHoldObject
  ;[0.09896 0.02986 0] Placement Mode: called from Puzzle Object Master
  (CallFunction|SetPlacementModeEnabled true)
  (Default|SetPlacementMode (Variables|Default|GetBP_PlayerCharacter) true)
  (Components|Activation|Deactivate (Variables|/Script/Engine.Character|GetCharacterMovement (Variables|Default|GetBP_PlayerCharacter))))

(event Input|ActionEvents|InputActionMouseLeftClick
  (params (Key :type Key%20Structure :default "None"))
  (:Pressed
    (if (Variables|Default|GetisPlacementModeEnabled)
      (Variables|Default|GetploppableActor
        (:then
          (Actor|DestroyActor (Variables|Default|GetploppableActor)))
        (:else
          _))
      (Class|BPIMoveable|MoveObjectPosition(Message) (Variables|/Game/LunarLabyrinth/Core/Characters/Player/Blueprints/BP_ThirdPersonCharacter.BP_ThirdPersonCharacter_C|GettempInteractable (Variables|Default|GetBP_PlayerCharacter)) (Variables|Default|GetClosest%20Grid%20Output) self))))

(fn ConstructionScript
  (bind _outactors (Actor|GetAllActorsOfClass "/Game/LunarLabyrinth/Core/Grid/BP_GridManager.BP_GridManager_C"))
  (Variables|Default|SetgridManager (Utilities|Array|Get(acopy) _outactors)))

(fn GrabObject
  (bind _bp_playercharacter (Variables|Default|GetBP_PlayerCharacter))
  (bind _rootcomponent (Variables|/Script/Engine.Actor|GetRootComponent _bp_playercharacter))
  (bind _returnvalue (Transformation|GetWorldLocation _rootcomponent))
  (if true
    (bind (_outhit _returnvalue_2) (Collision|LineTraceByChannel _returnvalue (+ _returnvalue (* (Math|Vector|GetForwardVector (Transformation|GetWorldRotation (Variables|/Script/Engine.Actor|GetRootComponent _bp_playercharacter))) 5e+02)) "TraceTypeQuery1" false 0 "None"))
    (if _returnvalue_2
      (Physics|Components|PhysicsHandle|GrabComponentatLocationwithRotation (Variables|Default|GetPhysicsHandle) (.HitComponent (Collision|BreakHitResult _outhit)) "None" (Transformation|GetWorldLocation (.HitComponent (Collision|BreakHitResult _outhit))) "0, 0, 0")
      (Variables|Default|Setobject%20is%20grabbed%20? true))))

(fn SetPlacementModeEnabled
  (params (IsEnabled :type Boolean))
  (bind _output_get (Variables|Default|SetisPlacementModeEnabled IsEnabled))
  (if _output_get
    (bind _returnvalue (Game|SpawnActorfromClass (Variables|Default|GetPloppableActorType) (Math|Transform|MakeTransform "0.000000,-100.000000,0.000000") "Undefined" "MultiplyWithRoot" 0 0))
    (bind _output_get_2 (Variables|Default|SetploppableActor _returnvalue))
    (Utilities|IsValid (Actor|GetComponentbyClass _output_get_2 "/Game/LunarLabyrinth/Core/Interactables/BP_Clickable.BP_Clickable_C")
      (:Is%20Valid
        (Default|InPlacementMode (Actor|GetComponentbyClass _output_get_2 "/Game/LunarLabyrinth/Core/Interactables/BP_Clickable.BP_Clickable_C")))
      (:Is%20Not%20Valid
        _))
    (AddComponent|AddACPloppableComponent _output_get_2)
    (else
      (bind _ploppableactor (Variables|Default|GetploppableActor)
        (:then
          (Actor|DestroyActor _ploppableactor))
        (:else)))))

(fn UpdatePlacement
  (bind (_worldlocation _worlddirection) (Game|Player|ConvertMouseLocationToWorldSpace))
  (bind _outhit (Collision|LineTraceByChannel _worldlocation (+ _worldlocation (* _worlddirection 1e+04)) "TraceTypeQuery3" false 0 "ForDuration"))
  (if (.bBlockingHit (Collision|BreakHitResult _outhit))
    (bind _closest_grid_output (Default|Getclosestgrid (Variables|Default|GetgridManager) (.Location (Collision|BreakHitResult _outhit))))
    (bind _output_get (Variables|Default|SetClosest%20Grid%20Output _closest_grid_output))
    (Transformation|SetActorLocation (Variables|Default|GetploppableActor) _output_get false false)))

(fn Spawn
  (bind _ploppableactor (Variables|Default|GetploppableActor))
  (bind _returnvalue (Actor|GetComponentbyClass _ploppableactor "/Game/LunarLabyrinth/Core/Interactables/AC_PloppableComponent.AC_PloppableComponent_C"))
  (Utilities|IsValid _returnvalue
    (:Is%20Valid
      (if (Variables|/Game/LunarLabyrinth/Core/Interactables/AC_PloppableComponent.AC_PloppableComponent_C|GetIsPlacementValid%20? _returnvalue)
        (Game|SpawnActorfromClass (Variables|Default|GetPloppableActorType) (Transformation|GetActorTransform (Variables|Default|GetploppableActor)) "AlwaysSpawn" "MultiplyWithRoot" 0 0)
        (CallFunction|SetPlacementModeEnabled false)
        (Default|SetPlacementMode (Variables|Default|GetBP_PlayerCharacter) false)))))

(fn SetTempInteractable
  (params (interactableActor :type Actor%20Object%20Reference))
  (Variables|Default|SetTempInteractable interactableActor))

(fn IsInteractable
  (return false))