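; BP_ReflectableObject is a light ray source object that feeds a ray origin and direction to its ACReflectableComponent.
; Construction applies the component's mesh and material to LightRaySourceModel and copies LightRayStartPos's world location and forward vector into the component.
; A looping timer started at BeginPlay re-copies them when its change check passes.
; That check compares cached location against the forward vector, and never refreshes its cached values.
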(event Custom|UpdateRayLoc
  (bind _lightraystartpos (Variables|Default|GetLightRayStartPos))
  (if (or (Utilities|Operators|NotEqual(!=) (Variables|Default|GetOldLoc) (Math|Vector|GetForwardVector _lightraystartpos) 0.0) (Utilities|Operators|NotEqual(!=) (Variables|Default|GetOldFwdVec) (Math|Vector|GetForwardVector _lightraystartpos) 0.0))
    (CallFunction|SetReflectableCompLoc)))

(event EventBeginPlay
  (bind _lightraystartpos (Variables|Default|GetLightRayStartPos))
  (Variables|Default|SetOldLoc (Transformation|GetWorldLocation _lightraystartpos))
  (Variables|Default|SetOldFwdVec (Math|Vector|GetForwardVector _lightraystartpos))
  (Utilities|Time|SetTimerbyEvent (delegate Custom|UpdateRayLoc) 0.05 true))

(fn ConstructionScript
  (CallFunction|InitializeReflectableComponent))

(fn InitializeReflectableComponent
  (bind _ac_reflectablecomponent (Variables|Default|GetAC_ReflectableComponent))
  (Utilities|FlowControl|Sequence
    (:then_0
      ;[0.01005 0.01042 0 0.906] Set ReflectableComponent Mesh
      (Components|StaticMesh|SetStaticMesh (Variables|Default|GetLightRaySourceModel) (Variables|/Game/AC_ReflectableComponent.AC_ReflectableComponent_C|GetreflectableMesh _ac_reflectablecomponent))
      (Rendering|Material|SetMaterial (Variables|Default|GetLightRaySourceModel) 0 (Variables|/Game/AC_ReflectableComponent.AC_ReflectableComponent_C|GetreflectableMeshMat _ac_reflectablecomponent)))
    (:then_1
      (CallFunction|SetReflectableCompLoc))))

(fn SetReflectableCompLoc
  (bind _ac_reflectablecomponent (Variables|Default|GetAC_ReflectableComponent))
  ;[0.01005 0.01042 0 0.906] Set Ray StartPoint
  (Variables|/Game/AC_ReflectableComponent.AC_ReflectableComponent_C|SetrayStartWorldLoc _ac_reflectablecomponent (Transformation|GetWorldLocation (Variables|Default|GetLightRayStartPos)))
  (Variables|/Game/AC_ReflectableComponent.AC_ReflectableComponent_C|SetrayStartFwdRot _ac_reflectablecomponent (Math|Vector|GetForwardVector (Variables|Default|GetLightRayStartPos))))