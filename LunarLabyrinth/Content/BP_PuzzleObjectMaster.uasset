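; Master Blueprint for puzzle objects, configuring each object's mesh and capabilities in its construction script.
; It applies ObjModel to the Model mesh and sets IsInteractable by testing for IF_Interactable, which subclasses implement manually.
; Objects flagged moveable or rotateable get an ACMoveableComponent added at construction, with the object passed in as its derived object.
; The event graph holds no active logic.
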(event EventBeginPlay)

(event Collision|EventActorBeginOverlap
  (params (OtherActor :type Actor%20Object%20Reference)))

(event EventTick
  (params (DeltaSeconds :type Float%20%28single-precision%29)))

(fn ConstructionScript
  (Utilities|FlowControl|Sequence
    (:then_0
      (CallFunction|InitializePuzzleObj))
    (:then_1
      (CallFunction|CheckInteractable))
    (:then_2
      (CallFunction|CheckMoveable))))

(fn CheckInteractable
  ;[0.2805 0.2917 0.2188] Interface is manually implemented in the sub classes of PuzzleObjectMaster
  (Variables|Default|SetisInteractable (Utilities|DoesObjectImplementInterface self "/Game/IF_Interactable.IF_Interactable_C")))

(fn InitializePuzzleObj
  ;[0.01005 0.01042 0 0.906] Set ReflectableComponent Mesh
  (Components|StaticMesh|SetStaticMesh (Variables|Default|GetModel) (Variables|Default|GetobjModel)))

(fn CheckMoveable
  (if (or (Variables|Default|GetisMoveable) (Variables|Default|GetIsRotateable))
    ;[0.01005 0.01042 0 0.906] Add & Init Moveable Comp
    (bind _returnvalue (AddComponent|AddACMoveableComponent))
    (bind _output_get (Variables|Default|SetAC_MoveableComp _returnvalue))
    (Default|SetDerivedObject _output_get self)
    (else
      (Variables|Default|SetisMoveable false))))